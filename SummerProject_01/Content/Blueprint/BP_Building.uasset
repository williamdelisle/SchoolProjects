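; Procedural building actor that assembles a single-storey rectangular room from modular static mesh pieces in the Construction Script, with no active runtime logic.
; When UpdateActive is set, it runs CreateWall, CreateFloor and CreateCeiling in sequence.
; CreateWall places corners and four wall runs sized by WallWidth and WallLengh, branching at DoorLocation on the first run.
; Floor and ceiling are tile grids spaced by WallObjectWidth, with the ceiling raised near WallObjectHeight.
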(fn `CreateCeiling`
  (bind _wallobjectwidth (`self.WallObjectWidth`))
  (for _index (range (+ (+ (`self.WallLengh`) 1) 1))
    (for _index_2 (range (+ (+ (`self.WallWidth`) 1) 1))
      (`AddComponent|NODE_AddStaticMeshComponent-15` :`RelativeTransform` (`KismetMathLibrary.MakeTransform` (`KismetMathLibrary.MakeVector` (`KismetMathLibrary.Conv_IntToDouble` (* _index_2 _wallobjectwidth)) (`KismetMathLibrary.Conv_IntToDouble` (* _index _wallobjectwidth)) (`KismetMathLibrary.Conv_IntToDouble` (- (`self.WallObjectHeight`) 10))) (struct :`Yaw` 90.0)))))
  (return))

(fn `CreateFloor`
  (bind _wallobjectwidth (`self.WallObjectWidth`))
  (for _index (range (+ (+ (`self.WallLengh`) 1) 1))
    (for _index_2 (range (+ (+ (`self.WallWidth`) 1) 1))
      (`AddComponent|NODE_AddStaticMeshComponent-13` :`RelativeTransform` (`KismetMathLibrary.MakeTransform` (`KismetMathLibrary.MakeVector` (`KismetMathLibrary.Conv_IntToDouble` (* _index_2 _wallobjectwidth)) (`KismetMathLibrary.Conv_IntToDouble` (* _index _wallobjectwidth))) (struct :`Yaw` 90.0)))))
  (return))

(fn `CreateWall`
  (bind _wallobjectwidth (`self.WallObjectWidth`))
  (bind _doorlocation (`self.DoorLocation`))
  (bind _wallobjectwidth_2 (`self.WallObjectWidth`))
  (for _index (range 1 (+ (`self.WallWidth`) 1))
    (for _index_2 (range _doorlocation 1)
      _)
    (if (== _doorlocation _index)
      (`AddComponent|NODE_AddStaticMeshComponent-7` :`RelativeTransform` (`KismetMathLibrary.MakeTransform` (`KismetMathLibrary.MakeVector` (`KismetMathLibrary.Conv_IntToDouble` (* _index_2 (`self.WallObjectWidth`))))))
      (else
        (`AddComponent|NODE_AddStaticMeshComponent-1` :`RelativeTransform` (`KismetMathLibrary.MakeTransform` (`KismetMathLibrary.MakeVector` (`KismetMathLibrary.Conv_IntToDouble` (* _index (`self.WallObjectWidth`)))))))))
  (`AddComponent|NODE_AddStaticMeshComponent-3` :`RelativeTransform` (`KismetMathLibrary.MakeTransform` (0.0 0.0 0.0) (struct :`Yaw` 90.0)))
  (for _index_3 (range 1 (+ (`self.WallLengh`) 1))
    (bind _returnvalue (* _index_3 (`self.WallObjectWidth`)))
    (`AddComponent|NODE_AddStaticMeshComponent-2` :`RelativeTransform` (`KismetMathLibrary.MakeTransform` (`KismetMathLibrary.MakeVector` 0.0 (`KismetMathLibrary.Conv_IntToDouble` _returnvalue)) (struct :`Yaw` 90.0))))
  (`AddComponent|NODE_AddStaticMeshComponent-4` :`RelativeTransform` (`KismetMathLibrary.MakeTransform` (`KismetMathLibrary.MakeVector` 0.0 (`KismetMathLibrary.Conv_IntToDouble` (* (+ (`self.WallLengh`) 2) (`self.WallObjectWidth`))))))
  (for _index_4 (range 1 (+ (`self.WallWidth`) 1))
    (bind _returnvalue_2 (* _index_4 _wallobjectwidth))
    (`AddComponent|NODE_AddStaticMeshComponent-8` :`RelativeTransform` (`KismetMathLibrary.MakeTransform` (`KismetMathLibrary.MakeVector` (`KismetMathLibrary.Conv_IntToDouble` _returnvalue_2) (`KismetMathLibrary.Conv_IntToDouble` (+ _returnvalue _wallobjectwidth))))))
  (`AddComponent|NODE_AddStaticMeshComponent-5` :`RelativeTransform` (`KismetMathLibrary.MakeTransform` (`KismetMathLibrary.MakeVector` (`KismetMathLibrary.Conv_IntToDouble` (* (+ (`self.WallWidth`) 2) (`self.WallObjectWidth`))) (`KismetMathLibrary.Conv_IntToDouble` (* (+ (`self.WallLengh`) 2) (`self.WallObjectWidth`)))) (struct :`Yaw` -90.0)))
  (for _index_5 (range 1 (+ (`self.WallLengh`) 1))
    (`AddComponent|NODE_AddStaticMeshComponent-9` :`RelativeTransform` (`KismetMathLibrary.MakeTransform` (`KismetMathLibrary.MakeVector` (`KismetMathLibrary.Conv_IntToDouble` (+ _returnvalue_2 _wallobjectwidth_2)) (`KismetMathLibrary.Conv_IntToDouble` (+ (* _index_5 _wallobjectwidth_2) _wallobjectwidth_2))) (struct :`Yaw` -90.0))))
  (`AddComponent|NODE_AddStaticMeshComponent-6` :`RelativeTransform` (`KismetMathLibrary.MakeTransform` (`KismetMathLibrary.MakeVector` (`KismetMathLibrary.Conv_IntToDouble` (* (+ (`self.WallWidth`) 2) (`self.WallObjectWidth`)))) (struct :`Yaw` 180.0))))

(fn `UserConstructionScript`
  (if (`self.Update Active`)
    (`|ExecutionSequence`
      (:`then_0`
        (`self.CreateWall`))
      (:`then_1`
        (`self.CreateFloor`))
      (:`then_2`
        (`self.CreateCeiling`)))))