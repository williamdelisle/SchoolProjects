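; BP_Stairs is a procedural stairs actor that builds a repeated run of static mesh steps.
; The Construction Script loops from zero to Amount, adding a static mesh component per index at that index times the X, Y and Z offsets.
; Every step keeps zero rotation and unit scale, and the Event Graph holds no active logic.
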(fn `UserConstructionScript`
  (locals (NewLocalVar_0 :type "Actor Object Reference"))
  (for _index (range (+ (`self.Amount`) 1))
    (`AddComponent|NODE_AddStaticMeshComponent-0` :`RelativeTransform` (`KismetMathLibrary.MakeTransform` (`KismetMathLibrary.MakeVector` (* _index (`self.X`)) (* _index (`self.Y`)) (* _index (`self.Z`)))))))